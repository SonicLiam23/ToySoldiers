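; BP_WeaponMaster is a weapon Blueprint, apparently the base for the game's guns, that handles firing for the owning third-person character.
; FireWeapon switches on WeaponName, with Pistol A and Assault Rifle A sharing one path.
; That path spawns a projectile at the current weapon's Barrel socket, rotated toward the crosshair target.
; It then decrements the clip in the weapon stats struct and ends on a fire-rate Delay with nothing after it.
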(event `FireWeapon`
  (params (CrosshairTarget :type "Vector Structure"))
  (bind _asbp_third_person_character (cast `/Game/ThirdPerson/Blueprints/BP_ThirdPersonCharacter` (`self.GetOwner`)))
  (bind _currentweapon (`/Game/ThirdPerson/Blueprints/BP_ThirdPersonCharacter.GetCurrentWeapon` _asbp_third_person_character))
  (switch `/Game/_Project/Props/Weapons/Enum_WeaponName` (`self.WeaponName`)
    (:`NewEnumerator0`
      _)
    (:`NewEnumerator2`
      _))
  (bind _returnvalue_location (`KismetMathLibrary.BreakTransform` (`self.GetSocketTransform` (`/Game/ThirdPerson/Blueprints/BP_ThirdPersonCharacter.Current Weapon` _asbp_third_person_character) "Barrel" "RTS_World")))
  (`|SpawnActorFromClass` "/Game/Projectile/MyProjectileBase.MyProjectileBase_C" (`KismetMathLibrary.MakeTransform` _returnvalue_location (`KismetMathLibrary.FindLookAtRotation` _returnvalue_location CrosshairTarget)) "Undefined" "MultiplyWithRoot" _asbp_third_person_character _asbp_third_person_character)
  (bind _weaponstats_currentclip (break `/Game/_Project/Props/Weapons/S_WeaponData` (`/Game/_Project/Props/Weapons/BP_WeaponMaster.WeaponStats` _currentweapon)))
  (bind _structout (setmembers `/Game/_Project/Props/Weapons/S_WeaponData` :`StructRef` (`self.WeaponStats`) :`CurrentClip` (- _weaponstats_currentclip 1)))
  (set `/Game/_Project/Props/Weapons/BP_WeaponMaster.WeaponStats` _structout _currentweapon)
  (bind (_weaponstats_currentclip_2 _weaponstats_maxclip _weaponstats_reserveammo _weaponstats_firerate) (break `/Game/_Project/Props/Weapons/S_WeaponData` (`/Game/_Project/Props/Weapons/BP_WeaponMaster.WeaponStats` _currentweapon)))
  (`KismetSystemLibrary.Delay` _weaponstats_firerate))