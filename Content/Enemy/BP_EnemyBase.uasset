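; BP_EnemyBase is an enemy Blueprint that fires projectiles, takes damage and is destroyed on death.
; It calls SpawnProjectile on its BPProjectileSpawner every Tick, with no timing check in this graph.
; HealthComponent events drive the rest: damage prints the health percentage in red text, and death destroys the actor.
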(event `self.ReceiveTick`
  (params (DeltaSeconds :type "Float (single-precision)"))
  (`ProjectileSpawner.SpawnProjectile` (`self.BP_ProjectileSpawner`)))

(event `self.HealthComponent.OnTakeDamage`
  (params (DamageAmount :type "Float (single-precision)"))
  (`KismetSystemLibrary.PrintText` (`KismetTextLibrary.Conv_DoubleToText` (`HealthComponent.GetHealthPercentage` (`self.HealthComponent`)) "HalfToEven") true true (struct :`R` 1.0 :`B` 0.04055 :`A` 1.0)))

(event `self.HealthComponent.OnDeath`
  (`self.K2_DestroyActor`))

(fn `UserConstructionScript`
  (`parent.UserConstructionScript`))